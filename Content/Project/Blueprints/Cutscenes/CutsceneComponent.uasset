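; Cutscene component that plays camera transitions between main menu, level selection and settings screens, plus the game-start sequence.
; On BeginPlay it registers with MyGameMode, resets cutscene actors and, in the Main Menu level, views through the cutscene camera.
; Per-transition timelines move the camera, reversed for returns, then switch and fade menu screens, with a busy flag blocking overlaps.
; Game start triggers level transition, restoring player view and input on fade-out.
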(event Custom|UpdatePlayerControl
  (bind _gamemoderef (Variables|Default|GetGameModeRef))
  (bind _playerref (Default|GetPlayerRef _gamemoderef))
  (bind _currentcontroler (Class|IPlayer|GetPlayerControler(Message) _playerref))
  (Game|Player|SetViewTargetwithBlend _currentcontroler _playerref 0.0 "VTBlend_Linear" 0.0 false)
  (bind _menuuiref (Default|GetMenuUI _gamemoderef))
  (Default|UpdatePlayersInputMode _gamemoderef false _menuuiref)
  (Variables|Default|SetIsPlayingCustcene? false)
  (EventDispatchers|UnbindEventfromOnFadeOut (stale Custom|PlayMainMenuCutscenes _fadeuiref) (delegate Custom|UpdatePlayerControl)))

(event Custom|PlayMainMenuCutscenes
  (params (CutsceneSelected :type MenuTransitionsEnum%20Enum :default "NewEnumerator0"))
  (bind _gamemoderef (Variables|Default|GetGameModeRef))
  (if (not (Variables|Default|GetIsPlayingCustcene?))
    (Variables|Default|SetIsPlayingCustcene? true)
    (switch Utilities|FlowControl|Switch|SwitchonMenuTransitionsEnum CutsceneSelected
      (:NewEnumerator0
        (bind (_direction _moveplayer _movecamera _rotatecamera) (Timeline|FromMainMenuToLevelSelection PlayFromStart)
          (:Update
            (Transformation|SetActorLocationAndRotation (Variables|Default|GetCameraForCutscene) _movecamera (Math|Rotator|MakeRotator 0.0 (.y _rotatecamera) (.z _rotatecamera)) false true))
          (:Finished
            (bind _menuuiref (Default|GetMenuUI (Variables|Default|GetGameModeRef)))
            (Default|UpdateCurrentScreen _menuuiref (Variables|/Game/Project/Blueprints/UI/MenuUI.MenuUI_C|GetLevelSelectCanvas _menuuiref))
            (Default|FadeMenu _menuuiref "NewEnumerator0")
            (bind _duration (Default|GetFadeDuration _menuuiref))
            (Utilities|FlowControl|Delay _duration)
            (Variables|Default|SetIsPlayingCustcene? false))))
      (:NewEnumerator1
        (bind (_direction_2 _moveplayer_2 _movecamera_2 _rotatecamera_2) (Timeline|LevelSelectionToMainMenu ReverseFromEnd)
          (:Update
            (Transformation|SetActorLocationAndRotation (Variables|Default|GetCameraForCutscene) _movecamera_2 (Math|Rotator|MakeRotator 0.0 (.y _rotatecamera_2) (.z _rotatecamera_2)) false true))
          (:Finished
            (bind _menuuiref_2 (Default|GetMenuUI (Variables|Default|GetGameModeRef)))
            (Default|UpdateCurrentScreen _menuuiref_2 (Variables|/Game/Project/Blueprints/UI/MenuUI.MenuUI_C|GetMainMenuCanvas _menuuiref_2))
            (Default|FadeMenu _menuuiref_2 "NewEnumerator0")
            (bind _duration_2 (Default|GetFadeDuration _menuuiref_2))
            (Utilities|FlowControl|Delay _duration_2)
            (Variables|Default|SetIsPlayingCustcene? false))))
      (:NewEnumerator2
        (bind (_direction_3 _camerarotation _cameramovement) (Timeline|MainMenuToSettings PlayFromStart)
          (:Update
            (Transformation|SetActorLocationAndRotation (Variables|Default|GetCameraForCutscene) _cameramovement (Math|Rotator|MakeRotator 0.0 (.y _camerarotation) (.z _camerarotation)) false true))
          (:Finished
            (bind _menuuiref_3 (Default|GetMenuUI (Variables|Default|GetGameModeRef)))
            (Default|UpdateCurrentScreen _menuuiref_3 (Variables|/Game/Project/Blueprints/UI/MenuUI.MenuUI_C|GetConfigCanvas _menuuiref_3))
            (Default|FadeMenu _menuuiref_3 "NewEnumerator0")
            (bind _duration_3 (Default|GetFadeDuration _menuuiref_3))
            (Utilities|FlowControl|Delay _duration_3)
            (Variables|Default|SetIsPlayingCustcene? false))))
      (:NewEnumerator3
        (bind (_direction_4 _camerarotation_2 _cameramovement_2) (Timeline|SettingsToMainMenu ReverseFromEnd)
          (:Update
            (Transformation|SetActorLocationAndRotation (Variables|Default|GetCameraForCutscene) _cameramovement_2 (Math|Rotator|MakeRotator 0.0 (.y _camerarotation_2) (.z _camerarotation_2)) false true))
          (:Finished
            (bind _menuuiref_4 (Default|GetMenuUI (Variables|Default|GetGameModeRef)))
            (Default|UpdateCurrentScreen _menuuiref_4 (Variables|/Game/Project/Blueprints/UI/MenuUI.MenuUI_C|GetMainMenuCanvas _menuuiref_4))
            (Default|FadeMenu _menuuiref_4 "NewEnumerator0")
            (bind _duration_4 (Default|GetFadeDuration _menuuiref_4))
            (Utilities|FlowControl|Delay _duration_4)
            (Variables|Default|SetIsPlayingCustcene? false))))
      (:NewEnumerator4
        (bind (_direction_5 _cameramovment _camerarotation_3) (Timeline|StartGame PlayFromStart)
          (:Update
            (Transformation|SetActorLocationAndRotation (Variables|Default|GetCameraForCutscene) _cameramovment (Math|Rotator|MakeRotator 0.0 (.y _camerarotation_3) (.z _camerarotation_3)) false true))
          (:Finished
            (bind _fadeuiref (Default|GetFadeUI _gamemoderef))
            (EventDispatchers|BindEventtoOnFadeOut _fadeuiref (delegate Custom|UpdatePlayerControl))
            (bind _leveltoopen (Default|GetLeveltoOpen _gamemoderef))
            (Default|StartLevelTransitionSequence _gamemoderef _leveltoopen)
            (Default|MoveDoor (Variables|Default|GetElevatorForCutscenes) false)))))))

(event EventBeginPlay
  (CallFunction|ComponentSetup))

(fn ConstructionScript)

(fn ActivateCameraforCutscenesView
  (params (PlayerController :type Player%20Controller%20Object%20Reference) (BlendTime :type Float%20%28single-precision%29))
  (Game|Player|SetViewTargetwithBlend PlayerController (Variables|Default|GetCameraForCutscene) BlendTime "VTBlend_Linear" 0.0 false))

(fn ComponentSetup
  (bind _playermodelforcutscene (Variables|Default|GetPlayerModelForCutscene))
  (bind _cameraforcutscene (Variables|Default|GetCameraForCutscene))
  (bind _asmy_game_mode (Utilities|Casting|CastToMyGameMode (Game|GetGameMode)))
  (bind _output_get (Variables|Default|SetGameModeRef _asmy_game_mode))
  (Default|SetCurrentCutsceneComponent _output_get self)
  (Utilities|IsValid _playermodelforcutscene
    (:Is%20Valid
      (Default|ReturntoStartLocationandRotation _playermodelforcutscene))
    (:Is%20Not%20Valid
      _))
  (Utilities|IsValid _cameraforcutscene
    (:Is%20Valid
      (Default|ReturntoStartLocationandRotation _cameraforcutscene))
    (:Is%20Not%20Valid
      _))
  (bind _currentlvlname (Default|GetCurrentLevelName (Variables|Default|GetGameModeRef)))
  (switch name _currentlvlname
    (:MainMenu
      (bind _playerref (Default|GetPlayerRef (Variables|Default|GetGameModeRef)))
      (bind _currentcontroler (Class|IPlayer|GetPlayerControler(Message) _playerref))
      (CallFunction|ActivateCameraforCutscenesView _currentcontroler 0.0)
      (Default|MoveDoor (Variables|Default|GetElevatorForCutscenes) true))))