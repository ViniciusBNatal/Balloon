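; Laser turret prop that fires timed, lethal beams, either when a tagged target enters its detection area or continuously.
; Each shot aims and stretches the beam to a target in line of sight, or uses a fixed direction and range.
; A delay-driven loop ramps dynamic material glow through warm-up, fire, decay and sleep phases with turret audio.
; AttackTarget toggles the damage window, during which players overlapping the HitBox are killed.
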(event OnComponentBeginOverlap(DetectionArea)
  (params (OverlappedComponent :type Primitive%20Component%20Object%20Reference) (OtherActor :type Actor%20Object%20Reference) (OtherComp :type Primitive%20Component%20Object%20Reference) (OtherBodyIndex :type Integer) (bFromSweep :type Boolean) (SweepResult :type Hit%20Result%20Structure%20%28by%20ref%29))
  (if (Actor|ActorHasTag OtherActor (Variables|Default|GetTargetTag))
    (Variables|Default|SetTargetRef OtherActor)
    (Variables|Default|SetPlayerInside true)
    (if (not (Variables|Default|GetIsShooting))
      (CallFunction|Shoot))))

(event OnComponentEndOverlap(DetectionArea)
  (params (OverlappedComponent :type Primitive%20Component%20Object%20Reference) (OtherActor :type Actor%20Object%20Reference) (OtherComp :type Primitive%20Component%20Object%20Reference) (OtherBodyIndex :type Integer))
  (if (Actor|ActorHasTag OtherActor (Variables|Default|GetTargetTag))
    (Variables|Default|SetPlayerInside false)))

(event OnComponentBeginOverlap(HitBox)
  (params (OverlappedComponent :type Primitive%20Component%20Object%20Reference) (OtherActor :type Actor%20Object%20Reference) (OtherComp :type Primitive%20Component%20Object%20Reference) (OtherBodyIndex :type Integer) (bFromSweep :type Boolean) (SweepResult :type Hit%20Result%20Structure%20%28by%20ref%29))
  (if (Actor|ActorHasTag OtherActor "Player")
    (bind _output_get (Variables|Default|SetDamageTarget OtherActor))
    (if (Variables|Default|GetCanAttack?)
      (Class|IPlayer|KillPlayer(Message) _output_get))))

(event OnComponentEndOverlap(HitBox)
  (params (OverlappedComponent :type Primitive%20Component%20Object%20Reference) (OtherActor :type Actor%20Object%20Reference) (OtherComp :type Primitive%20Component%20Object%20Reference) (OtherBodyIndex :type Integer))
  (if (Actor|ActorHasTag OtherActor "Player")
    (Variables|Default|SetDamageTarget 0)))

(event Custom|Shoot
  (|ShootSequence))

(event Custom|UpdateLazerVisual
  (params (FadeType :type FadeEnum%20Enum :default "NewEnumerator0"))
  (|UpateLazeVisualSequence FadeType))

(event EventUpdateDebugAreaVisibility
  (params (IsVisible :type Boolean))
  (bind _output_get (Variables|Default|SetDebugVisibility IsVisible))
  (Rendering|SetVisibility (Variables|Default|GetDebugArea) _output_get false))

(event EventBeginPlay
  (bind _asmy_game_mode (Utilities|Casting|CastToMyGameMode (Game|GetGameMode)))
  (Variables|Default|SetGameModeRef _asmy_game_mode)
  (if (and (Variables|Default|GetShootRegardlesOfTarget) (not (Variables|Default|GetLookAtTarget)))
    (Collision|SetCollisionEnabled (Variables|Default|GetDetectionArea) "NoCollision")
    (Utilities|FlowControl|Delay (Variables|Default|GetShootStartDelay))
    (CallFunction|Shoot)))

(fn ConstructionScript
  (|CreateMaterialParamRef)
  (CallFunction|UpdateDebugAreaVisibility (Variables|Default|GetDebugVisibility)))