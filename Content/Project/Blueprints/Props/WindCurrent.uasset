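; WindCurrent is a prop that pushes overlapping actors along its up vector with a configurable wind force.
; Entering the area sends messages that raise the actor's max speed and apply an external speed; leaving sends a zero max speed and the opposite external speed.
; Tick spins the visual, and the construction script sets debug cube visibility.
; The code sizing the Niagara effect to the area never runs.
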(event OnComponentBeginOverlap(AreaOfEffect)
  (params (OverlappedComponent :type Primitive%20Component%20Object%20Reference) (OtherActor :type Actor%20Object%20Reference) (OtherComp :type Primitive%20Component%20Object%20Reference) (OtherBodyIndex :type Integer) (bFromSweep :type Boolean) (SweepResult :type Hit%20Result%20Structure%20%28by%20ref%29))
  (bind _windforce (Variables|Default|GetWindForce))
  (bind _maxspeed (Class|IPlayer|GetMaxSpeed(Message) OtherActor))
  (Class|IPlayer|UpdateMaxSpeed(Message) OtherActor (+ _maxspeed _windforce))
  (Class|IPlayer|UpdateExternalSpeed(Message) OtherActor (* (Math|Vector|GetUpVector (Variables|Default|GetDefaultSceneRoot)) _windforce)))

(event OnComponentEndOverlap(AreaOfEffect)
  (params (OverlappedComponent :type Primitive%20Component%20Object%20Reference) (OtherActor :type Actor%20Object%20Reference) (OtherComp :type Primitive%20Component%20Object%20Reference) (OtherBodyIndex :type Integer))
  (Class|IPlayer|UpdateMaxSpeed(Message) OtherActor 0.0)
  (Class|IPlayer|UpdateExternalSpeed(Message) OtherActor (* (* (Math|Vector|GetUpVector (Variables|Default|GetDefaultSceneRoot)) (Variables|Default|GetWindForce)) -1)))

(event EventUpdateDebugAreaVisibility
  (params (IsVisible :type Boolean))
  (bind _output_get (Variables|Default|SetDebugAreaVisibility IsVisible))
  (Rendering|SetVisibility (Variables|Default|GetCube) _output_get false))

(event EventTick
  (params (DeltaSeconds :type Float%20%28single-precision%29))
  (Transformation|AddLocalRotation (Variables|Default|GetVisual) (Math|Rotator|MakeRotator 0.0 0.0 (Variables|Default|GetRotationSpeed)) false false))

(fn ConstructionScript
  (CallFunction|UpdateDebugAreaVisibility (Variables|Default|GetDebugAreaVisibility)))