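; Helium cylinder prop that grants a helium state to any actor entering its trigger box.
; On overlap it messages that actor with the cylinder's world Z as base position, MaxZDistance as the height limit, and helium turned on.
; A debug cube's visibility follows DebugVisibility through the construction script.
; Movement-lock and visual-scaling nodes remain in the graph but never run.
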(event OnComponentBeginOverlap(Box)
  (params (OverlappedComponent :type Primitive%20Component%20Object%20Reference) (OtherActor :type Actor%20Object%20Reference) (OtherComp :type Primitive%20Component%20Object%20Reference) (OtherBodyIndex :type Integer) (bFromSweep :type Boolean) (SweepResult :type Hit%20Result%20Structure%20%28by%20ref%29))
  (Class|IPlayer|UpdateZDistance(Message) OtherActor (.z (Transformation|GetWorldLocation (Variables|Default|GetCylinder))) (Variables|Default|GetMaxZDistance))
  (Class|IPlayer|UpdateHelium(Message) OtherActor true))

(event EventUpdateDebugAreaVisibility
  (params (IsVisible :type Boolean))
  (bind _output_get (Variables|Default|SetDebugVisibility IsVisible))
  (Rendering|SetVisibility (Variables|Default|GetCube) _output_get false))

(fn ConstructionScript
  (CallFunction|UpdateDebugAreaVisibility (Variables|Default|GetDebugVisibility)))