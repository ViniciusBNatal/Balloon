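; Tutorial prop that shows an input prompt icon in a widget component when the player is nearby.
; A trigger box detects actors tagged Player and shows the icon on overlap, hiding it when they leave.
; An icon update component sets the PropInteractionUI widget to the configured input type.
; StartActive makes the prompt visible from BeginPlay.
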(event OnComponentBeginOverlap(Box)
  (params (OverlappedComponent :type Primitive%20Component%20Object%20Reference) (OtherActor :type Actor%20Object%20Reference) (OtherComp :type Primitive%20Component%20Object%20Reference) (OtherBodyIndex :type Integer) (bFromSweep :type Boolean) (SweepResult :type Hit%20Result%20Structure%20%28by%20ref%29))
  (if (Actor|ActorHasTag OtherActor "Player")
    (bind _asprop_interaction_ui (Utilities|Casting|CastToPropInteractionUI (UserInterface|GetWidget (Variables|Default|GetInteractionBtnIcon))))
    (Default|UpdateIcon (Variables|Default|GetIconUpdateComponent) (Variables|Default|GetInputType) _asprop_interaction_ui true)))

(event OnComponentEndOverlap(Box)
  (params (OverlappedComponent :type Primitive%20Component%20Object%20Reference) (OtherActor :type Actor%20Object%20Reference) (OtherComp :type Primitive%20Component%20Object%20Reference) (OtherBodyIndex :type Integer))
  (if (Actor|ActorHasTag OtherActor "Player")
    (bind _asprop_interaction_ui (Utilities|Casting|CastToPropInteractionUI (UserInterface|GetWidget (Variables|Default|GetInteractionBtnIcon))))
    (Default|UpdateIcon (Variables|Default|GetIconUpdateComponent) (Variables|Default|GetInputType) _asprop_interaction_ui false)))

(event EventBeginPlay
  (if (Variables|Default|GetStartActive?)
    (bind _asprop_interaction_ui (Utilities|Casting|CastToPropInteractionUI (UserInterface|GetWidget (Variables|Default|GetInteractionBtnIcon))))
    (Default|UpdateIcon (Variables|Default|GetIconUpdateComponent) (Variables|Default|GetInputType) _asprop_interaction_ui true)))

(fn ConstructionScript)