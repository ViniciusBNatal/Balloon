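; Electric prop that applies a directional pull to a charged player inside its box area.
; Box overlaps or prop enter/exit events trigger it, using message calls to raise the player's max speed and add external speed along the root's negative up axis by PullForce.
; A ChargedPlayer flag prevents stacking and gates the reversal on exit.
; A cube shows the area for debugging, with visibility applied in the construction script.
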(event OnComponentBeginOverlap(Box)
  (params (OverlappedComponent :type Primitive%20Component%20Object%20Reference) (OtherActor :type Actor%20Object%20Reference) (OtherComp :type Primitive%20Component%20Object%20Reference) (OtherBodyIndex :type Integer) (bFromSweep :type Boolean) (SweepResult :type Hit%20Result%20Structure%20%28by%20ref%29))
  (Utilities|PlayerEnter OtherActor OtherActor OtherActor))

(event OnComponentEndOverlap(Box)
  (params (OverlappedComponent :type Primitive%20Component%20Object%20Reference) (OtherActor :type Actor%20Object%20Reference) (OtherComp :type Primitive%20Component%20Object%20Reference) (OtherBodyIndex :type Integer))
  (Utilities|PlayerExit OtherActor OtherActor))

(event EventUpdateDebugAreaVisibility
  (params (IsVisible :type Boolean))
  (bind _output_get (Variables|Default|SetDebugVisibility IsVisible))
  (Rendering|SetVisibility (Variables|Default|GetCube) _output_get false))

(event EventUpdateAction
  (params (PropEvent :type PropActionEventType%20Enum :default "NewEnumerator0") (CallOrigin :type Actor%20Object%20Reference))
  (switch Utilities|FlowControl|Switch|SwitchonPropActionEventType PropEvent
    (:NewEnumerator0
      (Utilities|PlayerEnter CallOrigin CallOrigin CallOrigin))
    (:NewEnumerator1
      (Utilities|PlayerExit CallOrigin CallOrigin))))

(fn ConstructionScript
  (CallFunction|UpdateDebugAreaVisibility (Variables|Default|GetDebugVisibility)))