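; IconUpdateComponent is a prop component that shows or hides an interaction icon widget with the image matching a given icon type.
; On BeginPlay it caches MyGameMode, whose interaction list maps icon types to images.
; UpdateIcon looks up the type in that list and passes the image to the icon's ChangeIcon, printing an error if none is found.
; When visibility is off, it simply sets the icon to Hidden.
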(event EventBeginPlay
  (bind _asmy_game_mode (Utilities|Casting|CastToMyGameMode (Game|GetGameMode)))
  (Variables|Default|SetMy%20Game%20Mode _asmy_game_mode))

(fn UpdateIcon
  (params (IconType :type InteractionIconTypes%20Enum :default "NewEnumerator0") (IconToChange :type Prop%20Interaction%20UI%20Object%20Reference) (IsVisible? :type Boolean))
  (if IsVisible?
    (bind _interactionsicondict (Default|GetInteractionList (Variables|Default|GetMy%20Game%20Mode)))
    (if (.ReturnValue (Utilities|Map|Find _interactionsicondict IconType))
      (Default|ChangeIcon IconToChange "SelfHitTestInvisible" (.Value (Utilities|Map|Find _interactionsicondict IconType)))
      (else
        (Development|PrintString "Enum Contains a Value Not Declarable" true false)))
    (else
      (Default|ChangeIcon IconToChange "Hidden"))))