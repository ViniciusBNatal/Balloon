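; A movable prop, with cart audio, that slides a set distance along its forward vector or gets shoved by the player.
; MoveObj runs a Delay-based loop of world offsets, slowing as it nears the target, and updates audio through the game mode's SoundManager; nothing here calls it.
; Player hits set physics velocity along the axis-rounded impact normal.
; The construction script draws the travel path as a debug line.
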(event OnComponentHit(Model)
  (params (HitComponent :type Primitive%20Component%20Object%20Reference) (OtherActor :type Actor%20Object%20Reference) (OtherComp :type Primitive%20Component%20Object%20Reference) (NormalImpulse :type Vector :default "0, 0, 0") (Hit :type Hit%20Result%20Structure%20%28by%20ref%29))
  (bind (_x _y _z) (Math|Vector|BreakVector (.impactnormal Hit)))
  (Utilities|Casting|CastToPlayer OtherActor)
  (Physics|SetPhysicsLinearVelocity (Variables|Default|GetModel) (* (Math|Vector|MakeVector (Math|Conversions|ToFloat(Integer) (Math|Float|Round _x)) (Math|Conversions|ToFloat(Integer) (Math|Float|Round _y)) (Math|Conversions|ToFloat(Integer) (Math|Float|Round _z))) (Variables|Default|GetVelocity)) false "None"))

(event Custom|MoveObj
  (bind _model (Variables|Default|GetModel))
  (bind _model_2 (Variables|Default|GetModel))
  (bind _returnvalue (Transformation|GetWorldLocation _model_2))
  (if (not (Variables|Default|GetIsMoving?))
    (Variables|Default|SetIsMoving? true)
    (Variables|Default|SetStartLocation _returnvalue)
    (Default|UpdateSound (Variables|/Game/Project/Blueprints/Managers/MyGameMode.MyGameMode_C|GetSoundManager (Variables|Default|GetGameModeRef)) (Variables|Default|GetCartAudio) "NewEnumerator0" 0.0 false)
    (Transformation|AddWorldOffset _model_2 (* (* (Math|Vector|GetForwardVector _model_2) (Variables|Default|GetVelocity)) (Math|Float|Clamp(Float) (/ (Math|Vector|VectorLength (- (+ (Variables|Default|GetStartLocation) (* (Math|Vector|GetForwardVector _model_2) (Variables|Default|GetDistance))) _returnvalue)) (Math|Vector|VectorLength (- (+ (Variables|Default|GetStartLocation) (* (Math|Vector|GetForwardVector _model_2) (Variables|Default|GetDistance))) (Variables|Default|GetStartLocation)))) 0.3)) false false :!label _label)
    (Utilities|FlowControl|Delay (Variables|Default|GetMovmentTick))
    (if (Math|Vector|Equal(Vector) (Transformation|GetWorldLocation _model) (+ (Variables|Default|GetStartLocation) (* (Math|Vector|GetForwardVector _model) (Variables|Default|GetDistance))) (Variables|Default|GetVelocity))
      (Variables|Default|SetIsMoving? false)
      (Default|UpdateSound (Variables|/Game/Project/Blueprints/Managers/MyGameMode.MyGameMode_C|GetSoundManager (Variables|Default|GetGameModeRef)) (Variables|Default|GetCartAudio) "NewEnumerator1" 0.5 false)
      (else
        (goto _label)))))

(event EventBeginPlay
  (bind _asmy_game_mode (Utilities|Casting|CastToMyGameMode (Game|GetGameMode)))
  (Variables|Default|SetGameModeRef _asmy_game_mode))

(fn ConstructionScript
  (bind _model (Variables|Default|GetModel))
  (bind _returnvalue (Transformation|GetWorldLocation _model))
  (Rendering|Debug|FlushPersistentDebugLines)
  (Rendering|Debug|DrawDebugLine _returnvalue (+ _returnvalue (* (Math|Vector|GetForwardVector _model) (Variables|Default|GetDistance))) "(R=1.000000,G=0.000000,B=0.000000,A=1.000000)" 1e+01 1e+01))