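; Player pawn that moves by applying physics forces to its static mesh, with horizontal and vertical movement plus controller-driven look.
; Move axes build direction vectors from control-rotation yaw only, and Tick applies their sum scaled by Speed as a force.
; While MoveUP or MoveDOWN is held, a Gate and Delay loop repeatedly pushes along the scene root's up axis at ZMovmentInterval.
; Rotate axes feed controller yaw and pitch input.
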(event EventTick
  (params (DeltaSeconds :type Float%20%28single-precision%29))
  (Physics|AddForce (Variables|Default|GetStaticMesh) (* (+ (Variables|Default|GetHorzMov) (Variables|Default|GetVertMov)) (Variables|Default|GetSpeed)) "None" false))

(event Input|ActionEvents|InputActionMoveUP
  (params (Key :type Key%20Structure :default "None"))
  ;[1 1 1] MovimentoZ
  (:Pressed
    (Utilities|FlowControl|Sequence
      (:then_0
        (goto _label Open))
      (:then_1
        (Utilities|FlowControl|Gate true :!label _label
          (:Exit
            (Physics|AddForce (Variables|Default|GetStaticMesh) (* (Math|Vector|GetUpVector (Variables|Default|GetDefaultSceneRoot)) (Variables|Default|GetUpForce)) "None" false)
            (Utilities|FlowControl|Delay (Variables|Default|GetZMovmentInterval))
            (goto _label))))))
  (:Released
    (goto _label Close)))

(event Input|ActionEvents|InputActionMoveDOWN
  (params (Key :type Key%20Structure :default "None"))
  ;[1 1 1] MovimentoZ
  (:Pressed
    (Utilities|FlowControl|Sequence
      (:then_0
        (goto _label Open))
      (:then_1
        (Utilities|FlowControl|Gate true :!label _label
          (:Exit
            (Physics|AddForce (Variables|Default|GetStaticMesh) (* (* (Math|Vector|GetUpVector (Variables|Default|GetDefaultSceneRoot)) (Variables|Default|GetDownForce)) -1.0) "None" false)
            (Utilities|FlowControl|Delay (Variables|Default|GetZMovmentInterval))
            (goto _label))))))
  (:Released
    (goto _label Close)))

(event Input|AxisEvents|InputAxisMoveHorizontal
  (params (AxisValue :type Float%20%28single-precision%29))
  ;[1 1 1] MovimentoXY
  (Variables|Default|SetHorzMov (* (Math|Vector|GetRightVector (Math|Rotator|MakeRotator 0.0 0.0 (.yaw (Pawn|GetControlRotation :!class /Script/Engine.Pawn)))) AxisValue)))

(event Input|AxisEvents|InputAxisMoveVertical
  (params (AxisValue :type Float%20%28single-precision%29))
  ;[1 1 1] MovimentoXY
  (Variables|Default|SetVertMov (* (Math|Vector|GetForwardVector (Math|Rotator|MakeRotator 0.0 0.0 (.yaw (Pawn|GetControlRotation :!class /Script/Engine.Pawn)))) AxisValue)))

(event Input|AxisEvents|InputAxisRotateHorizontal
  (params (AxisValue :type Float%20%28single-precision%29))
  ;[1 1 1] Rodar Camera
  (Pawn|Input|AddControllerYawInput AxisValue))

(event Input|AxisEvents|InputAxisRotateVertical
  (params (AxisValue :type Float%20%28single-precision%29))
  ;[1 1 1] Rodar Camera
  (Pawn|Input|AddControllerPitchInput AxisValue))

(fn ConstructionScript)