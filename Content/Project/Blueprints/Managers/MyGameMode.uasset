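; Game mode that acts as the game's central manager for level streaming, save data, UI and menu cutscenes.
; On BeginPlay it merges saved availability and start transforms into the level list, then builds a name-keyed dictionary that level updates write back to the save slot.
; Level transitions swap streamed levels on fade-out and reposition the player.
; Menu cutscenes blend registered cameras while a timeline moves a player model.
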(event Custom|Load/UnloadLevels
  (bind _fadeui (Variables|Default|GetFadeUI))
  (bind _leveltoopen (Variables|Default|GetLevelToOpen))
  (bind _levelsdict (Variables|Default|GetLevelsDict))
  (bind _leveltoopen_2 (Variables|Default|GetLevelToOpen))
  (bind _fadeui_2 (Variables|Default|GetFadeUI))
  (bind _playeractorref (Variables|Default|GetPlayerActorRef))
  (bind _returnvalue (Utilities|String|ToString(Name) _leveltoopen_2))
  (bind (_value _returnvalue_2) (Utilities|Map|Find _levelsdict _returnvalue))
  (bind (_levelname _isselectble _playerstartpoint _playerstartrotation) (Utilities|Struct|BreakLevelDataStruct _value))
  (if (Utilities|Name|Equal(Name) (Variables|Default|GetLevelToOpen) (Variables|Default|GetBaseLevelName))
    (if (Utilities|Name|Equal(Name) (Variables|Default|GetCurrentLevelName) "")
      _
      (else
        (Game|UnloadStreamLevel(byName) (Variables|Default|GetCurrentLevelName) true)))
    (Default|FadeIn/Out _fadeui_2 "NewEnumerator0")
    (EventDispatchers|UnbindEventfromOnFadeOut _fadeui_2 (delegate Custom|Load/UnloadLevels))
    (Variables|Default|SetCurrentLevelName "")
    (elif _returnvalue_2
      (bind _minscale (Class|IPlayer|GetMinScale(Message) _playeractorref))
      (Class|IPlayer|NewLevelStartup(Message) _playeractorref _playerstartpoint _playerstartrotation _minscale)
      (if (Utilities|Name|Equal(Name) (Variables|Default|GetCurrentLevelName) "")
        _
        (else
          (Game|UnloadStreamLevel(byName) (Variables|Default|GetCurrentLevelName) true)))
      (Game|LoadStreamLevel(byName) _leveltoopen true true)
      (Default|FadeIn/Out _fadeui "NewEnumerator0")
      (Variables|Default|SetCurrentLevelName _leveltoopen)
      (EventDispatchers|UnbindEventfromOnFadeOut _fadeui (delegate Custom|Load/UnloadLevels))
      (else
        (Default|FadeIn/Out (Variables|Default|GetFadeUI) "NewEnumerator0")
        (Development|PrintString (Utilities|String|Append "The Level " (Utilities|String|ToString(Name) _leveltoopen_2) " Doesnt exist in the LevelsList"))))))

(event Custom|PlayMainMenuCutscenes
  (params (CutsceneSelected :type MenuTransitionsEnum%20Enum :default "NewEnumerator0"))
  (if (not (Variables|Default|GetIsPlayingCustcene?))
    (Variables|Default|SetIsPlayingCustcene? true)
    (switch Utilities|FlowControl|Switch|SwitchonMenuTransitionsEnum CutsceneSelected
      (:NewEnumerator0
        (bind _cam (CallFunction|GetACameraforCutscene "MenuToElevator" false))
        (bind _currentcontroler (Class|IPlayer|GetPlayerControler(Message) (Variables|Default|GetPlayerActorRef)))
        (Game|Player|SetViewTargetwithBlend _currentcontroler _cam (Components|Timeline|GetTimelineLength (Variables|Default|GetMenu%20To%20Level%20selection)) "VTBlend_Linear" 0.0 false)
        (bind _moveplayer (Timeline|Menu%20To%20Level%20selection Play)
          (:Update
            (Transformation|SetActorLocation (Variables|Default|GetPlayerModelForCutscenes) _moveplayer false true))
          (:Finished
            (Variables|Default|SetIsPlayingCustcene? false)
            (bind _cam_2 (CallFunction|GetACameraforCutscene "ElevatorToLevelSelector" false))
            (bind _currentcontroler_2 (Class|IPlayer|GetPlayerControler(Message) (Variables|Default|GetPlayerActorRef)))
            (Game|Player|SetViewTargetwithBlend _currentcontroler_2 _cam_2 1.0 "VTBlend_Linear" 0.0 false)
            (Utilities|FlowControl|Delay 1.0)
            (CallFunction|FadeMenu "NewEnumerator0")))))))

(event EventBeginPlay
  (bind _savedataref (CallFunction|LoadSave))
  (if (== _savedataref 0)
    _
    (else
      (|PopulateLevelsList_2 (.LevelsAvaliable (Utilities|Struct|BreakSaveGameDataStructure (Variables|/Game/Project/Blueprints/Data/SaveData.SaveData_C|GetGameData _savedataref))) (.LevelsStartLocation (Utilities|Struct|BreakSaveGameDataStructure (Variables|/Game/Project/Blueprints/Data/SaveData.SaveData_C|GetGameData _savedataref))) (.LevelsStartRotation (Utilities|Struct|BreakSaveGameDataStructure (Variables|/Game/Project/Blueprints/Data/SaveData.SaveData_C|GetGameData _savedataref)))
        (:Exec2
          _))))
  (Utilities|PopulateLevelsDictionary))

(fn ConstructionScript)

(fn UpdateLevelSelectionState
  (params (LevelData :type Level%20Data%20Struct%20Structure) (UpdateIsSelectable? :type Boolean) (UpdatePlayerStartPoint? :type Boolean) (UpdatePlayerStartRotation? :type Boolean))
  (bind _levelname (Utilities|Struct|BreakLevelDataStruct LevelData))
  (bind (_levelname_2 _isselectble _playerstartpoint _playerstartrotation) (Utilities|Struct|BreakLevelDataStruct LevelData))
  (bind _levelsdict (Variables|Default|GetLevelsDict))
  (bind (_value _returnvalue) (Utilities|Map|Find _levelsdict _levelname))
  (if _returnvalue
    (LocalVariables|SetNewData (|Copy _value))
    (Utilities|FlowControl|Sequence
      (:then_0
        (if UpdateIsSelectable?
          (LocalVariables|SetNewData (Utilities|Struct|MakeLevelDataStruct (.levelname (LocalVariables|GetNewData)) _isselectble (.playerstartpoint (LocalVariables|GetNewData)) (.playerstartrotation (LocalVariables|GetNewData))))))
      (:then_1
        (if UpdatePlayerStartPoint?
          (LocalVariables|SetNewData (Utilities|Struct|MakeLevelDataStruct (.levelname (LocalVariables|GetNewData)) (.isselectble (LocalVariables|GetNewData)) _playerstartpoint (.playerstartrotation (LocalVariables|GetNewData))))))
      (:then_2
        (if UpdatePlayerStartRotation?
          (LocalVariables|SetNewData (Utilities|Struct|MakeLevelDataStruct (.levelname (LocalVariables|GetNewData)) (.isselectble (LocalVariables|GetNewData)) (.playerstartpoint (LocalVariables|GetNewData)) _playerstartrotation))))
      (:then_3
        (Utilities|Map|Add (Variables|Default|GetLevelsDict) (.LevelName (Utilities|Struct|BreakLevelDataStruct (LocalVariables|GetNewData))) (LocalVariables|GetNewData)))
      (:then_4
        (CallFunction|SaveGameplayData)))
    (else
      (Development|PrintString (Utilities|String|Append "The level: " _levelname " Doesn't exist in the dictionary") true true "(R=0.000000,G=0.660000,B=1.000000,A=1.000000)" 1e+01))))

(fn CreateUI
  (params (playerController :type Player%20Controller%20Object%20Reference))
  (Utilities|FlowControl|Sequence
    (:then_0
      ;[1 1 1] Cria Menu UI
      (if (== (Variables|Default|GetMenuUI) 0)
        (bind _returnvalue (UserInterface|CreateWidget "/Game/Project/Blueprints/UI/MenuUI.MenuUI_C" playerController))
        (bind _output_get (Variables|Default|SetMenuUI _returnvalue))
        (UserInterface|Viewport|AddtoViewport _output_get 0)
        (else
          (Development|PrintString "Menu UI Already Exists" true false "(R=0.000000,G=0.660000,B=1.000000,A=1.000000)" 5.0))))
    (:then_1
      ;[1 1 1] Cria Fade UI
      (if (== (Variables|Default|GetFadeUI) 0)
        (bind _returnvalue_2 (UserInterface|CreateWidget "/Game/Project/Blueprints/UI/FadeUI.FadeUI_C" playerController))
        (bind _output_get_2 (Variables|Default|SetFadeUI _returnvalue_2))
        (UserInterface|Viewport|AddtoViewport _output_get_2 0)
        (Default|FadeIn/Out _output_get_2 "NewEnumerator0")
        (else
          (Development|PrintString "Fade UI Already Exists" true false "(R=0.000000,G=0.660000,B=1.000000,A=1.000000)" 5.0))))
    (:then_2
      ;[1 1 1] Cria Pause UI
      (if (== (Variables|Default|GetPauseUI) 0)
        (bind _returnvalue_3 (UserInterface|CreateWidget "/Game/Project/Blueprints/UI/PauseUI.PauseUI_C" playerController))
        (bind _output_get_3 (Variables|Default|SetPauseUI _returnvalue_3))
        (UserInterface|Viewport|AddtoViewport _output_get_3 0)
        (else
          (Development|PrintString "Pause UI Already Exists" true false "(R=0.000000,G=0.660000,B=1.000000,A=1.000000)" 5.0))))
    (:then_3
      (return))))

(fn GetLevelsList
  (return (Variables|Default|GetLevelsList)))

(fn SaveGameplayData
  (bind _levelsdict (Variables|Default|GetLevelsDict))
  (bind _levelsdict_2 (Variables|Default|GetLevelsDict))
  (if (!= (Variables|Default|GetSaveData) 0)
    (bind _index (Utilities|FlowControl|ForLoopwithBreak 0 (- (Utilities|Map|Length _levelsdict_2) 1))
      (:LoopBody
        (Utilities|Array|SetArrayElem (.LevelsAvaliable (Utilities|Struct|BreakSaveGameDataStructure (Variables|/Game/Project/Blueprints/Data/SaveData.SaveData_C|GetGameData (Variables|Default|GetSaveData)))) _index (.isSelectble (Utilities|Struct|BreakLevelDataStruct (.Value (Utilities|Map|Find _levelsdict_2 (.levelname (Utilities|Array|Get(acopy) (Variables|Default|GetLevelsList) _index)))))))
        (Utilities|Array|SetArrayElem (.LevelsStartLocation (Utilities|Struct|BreakSaveGameDataStructure (Variables|/Game/Project/Blueprints/Data/SaveData.SaveData_C|GetGameData (Variables|Default|GetSaveData)))) _index (.PlayerStartPoint (Utilities|Struct|BreakLevelDataStruct (.Value (Utilities|Map|Find _levelsdict_2 (.levelname (Utilities|Array|Get(acopy) (Variables|Default|GetLevelsList) _index)))))))
        (Utilities|Array|SetArrayElem (.LevelsStartRotation (Utilities|Struct|BreakSaveGameDataStructure (Variables|/Game/Project/Blueprints/Data/SaveData.SaveData_C|GetGameData (Variables|Default|GetSaveData)))) _index (.PlayerStartRotation (Utilities|Struct|BreakLevelDataStruct (.Value (Utilities|Map|Find _levelsdict_2 (.levelname (Utilities|Array|Get(acopy) (Variables|Default|GetLevelsList) _index))))))))
      (:Completed
        (SaveGame|SaveGametoSlot (Variables|Default|GetSaveData) (Variables|/Game/Project/Blueprints/Data/SaveData.SaveData_C|GetSaveSlot (Variables|Default|GetSaveData)))))
    (else
      (bind _returnvalue (SaveGame|CreateSaveGameObject "/Game/Project/Blueprints/Data/SaveData.SaveData_C"))
      (bind _output_get (Variables|Default|SetSaveData _returnvalue))
      (Variables|/Game/Project/Blueprints/Data/SaveData.SaveData_C|SetSaveSlot _output_get (Variables|Default|GetSaveSlotSelected))
      (bind _index_2 (Utilities|FlowControl|ForLoopwithBreak 0 (- (Utilities|Map|Length _levelsdict) 1))
        (:LoopBody
          (Utilities|Array|Add (.LevelsAvaliable (Utilities|Struct|BreakSaveGameDataStructure (Variables|/Game/Project/Blueprints/Data/SaveData.SaveData_C|GetGameData _output_get))) (.isSelectble (Utilities|Struct|BreakLevelDataStruct (.Value (Utilities|Map|Find _levelsdict (.levelname (Utilities|Array|Get(acopy) (Variables|Default|GetLevelsList) _index_2)))))))
          (Utilities|Array|Add (.LevelsStartLocation (Utilities|Struct|BreakSaveGameDataStructure (Variables|/Game/Project/Blueprints/Data/SaveData.SaveData_C|GetGameData _output_get))) (.PlayerStartPoint (Utilities|Struct|BreakLevelDataStruct (.Value (Utilities|Map|Find _levelsdict (.levelname (Utilities|Array|Get(acopy) (Variables|Default|GetLevelsList) _index_2)))))))
          (Utilities|Array|Add (.LevelsStartRotation (Utilities|Struct|BreakSaveGameDataStructure (Variables|/Game/Project/Blueprints/Data/SaveData.SaveData_C|GetGameData _output_get))) (.PlayerStartRotation (Utilities|Struct|BreakLevelDataStruct (.Value (Utilities|Map|Find _levelsdict (.levelname (Utilities|Array|Get(acopy) (Variables|Default|GetLevelsList) _index_2))))))))
        (:Completed
          (SaveGame|SaveGametoSlot _output_get (Variables|/Game/Project/Blueprints/Data/SaveData.SaveData_C|GetSaveSlot _output_get)))))))

(fn LoadSave
  (bind _returnvalue (SaveGame|LoadGamefromSlot (Variables|Default|GetSaveSlotSelected)))
  (bind _assave_data (Utilities|Casting|CastToSaveData _returnvalue))
  (bind _output_get (Variables|Default|SetSaveData _assave_data))
  (return _output_get))

(fn SavePlayerRef
  (params (Player :type Pawn%20Object%20Reference))
  (if (Utilities|IsValid (Variables|Default|GetPlayerActorRef))
    (Actor|DestroyActor Player)
    (return false)
    (else
      (Variables|Default|SetPlayerActorRef Player)
      (return true))))

(fn GetLevelsDictionary
  (return (Variables|Default|GetLevelsDict)))

(fn GetPlayerRef
  (return (Variables|Default|GetPlayerActorRef)))

(fn GetBaseLevelName
  (return (Variables|Default|GetBaseLevelName)))

(fn StartLevelTransitionSequence
  (params (LevelName :type Name))
  (bind _fadeui (Variables|Default|GetFadeUI))
  (Variables|Default|SetLevelToOpen LevelName)
  (EventDispatchers|BindEventtoOnFadeOut _fadeui (EventDispatchers|CreateEvent :!event Custom|Load/UnloadLevels))
  (Default|FadeIn/Out _fadeui "NewEnumerator1"))

(fn GetMenuUI
  (return (Variables|Default|GetMenuUI)))

(fn GetFadeUI
  (return (Variables|Default|GetFadeUI)))

(fn UiSetup
  (CallFunction|CreateUI (Game|GetPlayerController 0))
  (bind _returnvalue (Game|GetCurrentLevelName true))
  (CallFunction|UpdatePlayersInputMode (Utilities|Enum|Equal(Enum) _returnvalue (Utilities|String|ToString(Name) (Variables|Default|GetBaseLevelName))) (Variables|Default|GetMenuUI)))

(fn GetCurrentLevelName
  (return (Variables|Default|GetCurrentLevelName)))

(fn SaveSettingsData
  (bind _menuui (Variables|Default|GetMenuUI))
  (bind _menuui_2 (Variables|Default|GetMenuUI))
  (if (!= (Variables|Default|GetSaveData) 0)
    (Variables|/Game/Project/Blueprints/Data/SaveData.SaveData_C|SetSettingsData (Variables|Default|GetSaveData) (Utilities|Struct|MakeSaveSettingsDataStructure (Class|CheckBox|IsChecked (Variables|/Game/Project/Blueprints/UI/MenuUI.MenuUI_C|GetWindowedCheckBox _menuui_2)) (Class|Slider|GetValue (Variables|/Game/Project/Blueprints/UI/MenuUI.MenuUI_C|GetMusicSlider _menuui_2)) (Class|Slider|GetValue (Variables|/Game/Project/Blueprints/UI/MenuUI.MenuUI_C|GetSFXSlider _menuui_2)) (Class|ComboBoxString|GetSelectedIndex (Variables|/Game/Project/Blueprints/UI/MenuUI.MenuUI_C|GetResolutionDropDown _menuui_2))))
    (Variables|/Game/Project/Blueprints/Data/SaveData.SaveData_C|SetSaveSlot (Variables|Default|GetSaveData) (Variables|Default|GetSaveSlotSelected))
    (SaveGame|SaveGametoSlot (Variables|Default|GetSaveData) (Variables|/Game/Project/Blueprints/Data/SaveData.SaveData_C|GetSaveSlot (Variables|Default|GetSaveData)))
    (else
      (bind _returnvalue (SaveGame|CreateSaveGameObject "/Game/Project/Blueprints/Data/SaveData.SaveData_C"))
      (bind _output_get (Variables|Default|SetSaveData _returnvalue))
      (Variables|/Game/Project/Blueprints/Data/SaveData.SaveData_C|SetSaveSlot _output_get (Variables|Default|GetSaveSlotSelected))
      (Variables|/Game/Project/Blueprints/Data/SaveData.SaveData_C|SetSettingsData _output_get (Utilities|Struct|MakeSaveSettingsDataStructure (Class|CheckBox|IsChecked (Variables|/Game/Project/Blueprints/UI/MenuUI.MenuUI_C|GetWindowedCheckBox _menuui)) (Class|Slider|GetValue (Variables|/Game/Project/Blueprints/UI/MenuUI.MenuUI_C|GetMusicSlider _menuui)) (Class|Slider|GetValue (Variables|/Game/Project/Blueprints/UI/MenuUI.MenuUI_C|GetSFXSlider _menuui)) (Class|ComboBoxString|GetSelectedIndex (Variables|/Game/Project/Blueprints/UI/MenuUI.MenuUI_C|GetResolutionDropDown _menuui))))
      (SaveGame|SaveGametoSlot _output_get (Variables|/Game/Project/Blueprints/Data/SaveData.SaveData_C|GetSaveSlot _output_get)))))

(fn GetSaveData
  (bind _savedata (Variables|Default|GetSaveData))
  (if (!= _savedata 0)
    (return _savedata)
    (else
      (Development|PrintString (Utilities|String|Append "There is No Save ata On The " (Variables|Default|GetSaveSlotSelected)) true false "(R=0.000000,G=0.660000,B=1.000000,A=1.000000)" 5.0)
      (return 0))))

(fn UpdatePlayersInputMode
  (params (IsInUI? :type Boolean) (WidgetToFocus :type User%20Widget%20Object%20Reference))
  (bind _returnvalue (Game|GetPlayerController 0))
  (if IsInUI?
    (Widget|SetVisibility WidgetToFocus "SelfHitTestInvisible")
    (Input|SetInputModeUIOnly _returnvalue WidgetToFocus "DoNotLock")
    (else
      (Widget|SetVisibility WidgetToFocus "Hidden")
      (Input|SetInputModeGameOnly _returnvalue)))
  (bind _playerref (CallFunction|GetPlayerRef))
  (Actor|Tick|SetActorTickEnabled _playerref (not IsInUI?))
  (Widget|SetIsEnabled WidgetToFocus IsInUI?)
  (Variables|/Script/Engine.PlayerController|SetbShowMouseCursor _returnvalue IsInUI?))

(fn UpdatePauseGame
  (Game|SetGamePaused (not (Game|IsGamePaused))))

(fn GetPauseUI
  (return (Variables|Default|GetPauseUI)))

(fn AddCameraforCutscenes
  (params (PlayerForCutscene :type Camera%20for%20Cutscenes%20Object%20Reference))
  (bind _returnvalue (Utilities|GetObjectName PlayerForCutscene))
  (bind _camerasforcutsceneref (Variables|Default|GetCamerasForCutsceneRef))
  (bind _returnvalue_2 (Class|KismetStringLibrary|ToUpper _returnvalue))
  (if (not (.ReturnValue (Utilities|Map|Find _camerasforcutsceneref _returnvalue_2)))
    (if (and (Variables|/Game/Project/Blueprints/Cutscenes/CameraForCutscenes.CameraForCutscenes_C|GetIsStartCamera? PlayerForCutscene) (not (Utilities|IsValid (Variables|Default|GetStartMenuCameraID))))
      _
      (else
        (Variables|/Game/Project/Blueprints/Cutscenes/CameraForCutscenes.CameraForCutscenes_C|SetIsStartCamera? PlayerForCutscene false)
        (Development|PrintString "More than 1 Start Camera In Scene")))
    (Utilities|Map|Add _camerasforcutsceneref _returnvalue_2 PlayerForCutscene)))

(fn SetPlayerModelforCutscenes
  (params (Model :type Actor%20Object%20Reference))
  (Variables|Default|SetPlayerModelForCutscenes Model))

(fn GetPlayerModelforCutscenes
  (return (Variables|Default|GetPlayerModelForCutscenes)))

(fn GetACameraforCutscene
  (params (CamID :type String) (GetStarterCamera? :type Boolean))
  (bind _returnvalue (Class|KismetStringLibrary|ToUpper CamID))
  (bind _camerasforcutsceneref (Variables|Default|GetCamerasForCutsceneRef))
  (bind (_value _returnvalue_2) (Utilities|Map|Find _camerasforcutsceneref _returnvalue))
  (if GetStarterCamera?
    (return (Variables|Default|GetStartMenuCameraID))
    (elif _returnvalue_2
      (return _value))))