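; Level transition actor with two sliding doors and a trigger box that sends the player to the configured level.
; On BeginPlay the doors animate open or closed per StartOpen, using a timed Delay loop of local offsets guarded against re-entry.
; Any overlap starts closing the doors, while a Player-tagged actor also has its game mode reference asked to start the transition sequence to LevelToOpen.
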(event OnComponentBeginOverlap(Box)
  (params (OverlappedComponent :type Primitive%20Component%20Object%20Reference) (OtherActor :type Actor%20Object%20Reference) (OtherComp :type Primitive%20Component%20Object%20Reference) (OtherBodyIndex :type Integer) (bFromSweep :type Boolean) (SweepResult :type Hit%20Result%20Structure%20%28by%20ref%29))
  (Utilities|FlowControl|Sequence
    (:then_0
      (CallFunction|MoveDoor false))
    (:then_1
      (if (Actor|ActorHasTag OtherActor "Player")
        (CallFunction|ChangeLevel OtherActor)))))

(event Custom|MoveDoor
  (params (IsOpening? :type Boolean))
  (bind _doorduration (Variables|Default|GetDoorDuration))
  (bind _doorduration_2 (Variables|Default|GetDoorDuration))
  (bind _doormaxdistance (Variables|Default|GetDoorMaxDistance))
  (bind _leftdoor (Variables|Default|GetLeftDoor))
  (bind _rightdoor (Variables|Default|GetRightDoor))
  (bind _leftdoor_2 (Variables|Default|GetLeftDoor))
  (bind _rightdoor_2 (Variables|Default|GetRightDoor))
  (bind _doormaxdistance_2 (Variables|Default|GetDoorMaxDistance))
  (bind _basedoorposition (Variables|Default|GetBaseDoorPosition))
  (bind _doormaxdistance_3 (Variables|Default|GetDoorMaxDistance))
  (bind _basedoorposition_2 (Variables|Default|GetBaseDoorPosition))
  (bind _returnvalue (/ 0.02 _doorduration))
  (bind _returnvalue_2 (/ 0.02 _doorduration_2))
  (bind _returnvalue_3 (- _doormaxdistance_2 _basedoorposition))
  (bind _returnvalue_4 (- _doormaxdistance_3 _basedoorposition_2))
  (bind _relativelocation (Variables|/Script/Engine.SceneComponent|GetRelativeLocation _rightdoor))
  (bind _relativelocation_2 (Variables|/Script/Engine.SceneComponent|GetRelativeLocation _leftdoor))
  (bind _relativelocation_3 (Variables|/Script/Engine.SceneComponent|GetRelativeLocation _leftdoor_2))
  (bind _relativelocation_4 (Variables|/Script/Engine.SceneComponent|GetRelativeLocation _rightdoor_2))
  (bind _returnvalue_5 (* _returnvalue_2 _returnvalue_4))
  (bind _returnvalue_6 (* _returnvalue _returnvalue_3))
  (if (not (Variables|Default|GetIsDoorMoving?))
    (Variables|Default|SetIsDoorMoving? true)
    (if IsOpening?
      (Transformation|SetRelativeLocation _leftdoor_2 (Math|Vector|MakeVector (Variables|Default|GetBaseDoorPosition) (.y _relativelocation_3) (.z _relativelocation_3)) false true)
      (Transformation|SetRelativeLocation _rightdoor_2 (Math|Vector|MakeVector (* -1 (Variables|Default|GetBaseDoorPosition)) (.y _relativelocation_4) (.z _relativelocation_4)) false true)
      (if (and (< (Math|Float|Absolute(Float) (.x (Variables|/Script/Engine.SceneComponent|GetRelativeLocation (Variables|Default|GetRightDoor)))) _doormaxdistance) (< (Math|Float|Absolute(Float) (.x (Variables|/Script/Engine.SceneComponent|GetRelativeLocation (Variables|Default|GetLeftDoor)))) _doormaxdistance)) :!label _label
        (Transformation|AddLocalOffset (Variables|Default|GetLeftDoor) (Math|Vector|MakeVector _returnvalue_5 0.0 0.0) false false)
        (Transformation|AddLocalOffset (Variables|Default|GetRightDoor) (Math|Vector|MakeVector (* -1 _returnvalue_5) 0.0 0.0) false false)
        (Utilities|FlowControl|Delay 0.02)
        (goto _label)
        (else
          (Variables|Default|SetIsDoorMoving? false)))
      (else
        (Transformation|SetRelativeLocation _leftdoor (Math|Vector|MakeVector (Variables|Default|GetDoorMaxDistance) (.y _relativelocation_2) (.z _relativelocation_2)) false true)
        (Transformation|SetRelativeLocation _rightdoor (Math|Vector|MakeVector (* -1 (Variables|Default|GetDoorMaxDistance)) (.y _relativelocation) (.z _relativelocation)) false true)
        (if (and (> (Math|Float|Absolute(Float) (.x (Variables|/Script/Engine.SceneComponent|GetRelativeLocation (Variables|Default|GetRightDoor)))) (* -1 (Variables|Default|GetBaseDoorPosition))) (> (Math|Float|Absolute(Float) (.x (Variables|/Script/Engine.SceneComponent|GetRelativeLocation (Variables|Default|GetLeftDoor)))) (Variables|Default|GetBaseDoorPosition))) :!label _label_2
          (Transformation|AddLocalOffset (Variables|Default|GetLeftDoor) (Math|Vector|MakeVector (* -1 _returnvalue_6) 0.0 0.0) false false)
          (Transformation|AddLocalOffset (Variables|Default|GetRightDoor) (Math|Vector|MakeVector _returnvalue_6 0.0 0.0) false false)
          (Utilities|FlowControl|Delay 0.02)
          (goto _label_2)
          (else
            (Variables|Default|SetIsDoorMoving? false)))))))

(event EventBeginPlay
  (CallFunction|MoveDoor (Variables|Default|GetStartOpen?)))

(fn ConstructionScript)

(fn ChangeLevel
  (params (ObjectInsideCollision :type Actor%20Object%20Reference))
  (bind _gmref (Class|IPlayer|GetGameModeRef(Message) ObjectInsideCollision))
  (Default|StartLevelTransitionSequence _gmref (Variables|Default|GetLevelToOpen)))