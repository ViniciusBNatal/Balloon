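; Test player pawn that moves a physics body in three axes, with controller-driven camera rotation.
; Camera-yaw-relative axis input feeds a speed-clamped velocity set and debug-printed each Tick, with linear damping raised when horizontal input is idle.
; Held up/down inputs run Gate and Delay loops that apply repeated forces; moving down also shrinks the Visual down to a minimum size.
; UpdateVisualScale also supports capped growth, and SetCharged stores a charge flag.
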(event EventTick
  (params (DeltaSeconds :type Float%20%28single-precision%29))
  (bind _aceleration (Variables|Default|GetAceleration))
  (bind _maxspeed (Variables|Default|GetMaxSpeed))
  (bind _horzmov (Variables|Default|GetHorzMov))
  (bind _vertmov (Variables|Default|GetVertMov))
  (bind _player (Variables|Default|GetPlayer))
  (bind _speed (Variables|Default|GetSpeed))
  (bind _returnvalue (Transformation|GetComponentVelocity _player))
  (bind _returnvalue_2 (* -1 _maxspeed))
  (bind _returnvalue_3 (+ _horzmov _vertmov))
  (bind _returnvalue_4 (* _returnvalue_3 _speed))
  (bind _returnvalue_5 (* _returnvalue_4 _aceleration))
  (bind _returnvalue_6 (+ _returnvalue _returnvalue_5))
  (bind _returnvalue_7 (Math|Vector|ClampVectorSize _returnvalue_6 _returnvalue_2 _maxspeed))
  (Physics|SetPhysicsLinearVelocity _player _returnvalue_7 false "None")
  (Development|PrintString (Utilities|String|ToString(Vector) _returnvalue_7)))

(event Input|ActionEvents|InputActionMoveUP
  (params (Key :type Key%20Structure))
  ;[1 1 1] MovimentoZ
  (:Pressed
    (Utilities|FlowControl|Sequence
      (:then_0
        (goto _label Open))
      (:then_1
        (Utilities|FlowControl|Gate true :!label _label
          (:Exit
            (Physics|AddForce (Variables|Default|GetPlayer) (* (Math|Vector|GetUpVector (Variables|Default|GetPlayer)) (Variables|Default|GetUpForce)) "None" false)
            (Utilities|FlowControl|Delay (Variables|Default|GetZMovmentInterval))
            (goto _label))))))
  (:Released
    (goto _label Close)))

(event Input|ActionEvents|InputActionMoveDOWN
  (params (Key :type Key%20Structure))
  ;[1 1 1] MovimentoZ
  (:Pressed
    (Utilities|FlowControl|Sequence
      (:then_0
        (goto _label Open))
      (:then_1
        (Utilities|FlowControl|Gate true :!label _label
          (:Exit
            (Physics|AddForce (Variables|Default|GetPlayer) (* (* (Math|Vector|GetUpVector (Variables|Default|GetPlayer)) (Variables|Default|GetDownForce)) -1.0) "None" false)
            (CallFunction|UpdateVisualScale false (Variables|Default|GetScaleReduction))
            (Utilities|FlowControl|Delay (Variables|Default|GetZMovmentInterval))
            (goto _label))))))
  (:Released
    (goto _label Close)))

(event Input|AxisEvents|InputAxisMoveHorizontal
  (params (AxisValue :type Float%20%28single-precision%29))
  ;[1 1 1] MovimentoXY
  (Variables|Default|SetHorzMov (* (Math|Vector|GetRightVector (Math|Rotator|MakeRotator 0.0 0.0 (.yaw (Pawn|GetControlRotation :!class /Script/Engine.Pawn)))) AxisValue))
  (Utilities|UpdateLinearDamping))

(event Input|AxisEvents|InputAxisMoveVertical
  (params (AxisValue :type Float%20%28single-precision%29))
  ;[1 1 1] MovimentoXY
  (Variables|Default|SetVertMov (* (Math|Vector|GetForwardVector (Math|Rotator|MakeRotator 0.0 0.0 (.yaw (Pawn|GetControlRotation :!class /Script/Engine.Pawn)))) AxisValue))
  (Utilities|UpdateLinearDamping))

(event Input|AxisEvents|InputAxisRotateHorizontal
  (params (AxisValue :type Float%20%28single-precision%29))
  ;[1 1 1] Rodar Camera
  (Pawn|Input|AddControllerYawInput AxisValue))

(event Input|AxisEvents|InputAxisRotateVertical
  (params (AxisValue :type Float%20%28single-precision%29))
  ;[1 1 1] Rodar Camera
  (Pawn|Input|AddControllerPitchInput AxisValue))

(fn ConstructionScript
  (Variables|Default|SetBaseLinearDamping (Class|PrimitiveComponent|GetLinearDamping (Variables|Default|GetPlayer))))

(fn UpdateVisualScale
  (params (Add? :type Boolean) (ScaleChange :type Float%20%28single-precision%29))
  (bind _maxsizepossible (Variables|Default|GetMaxSizePossible))
  (bind _visual (Variables|Default|GetVisual))
  (bind _minsizepossible (Variables|Default|GetMinSizePossible))
  (bind _returnvalue (Transformation|GetWorldScale _visual))
  (bind _returnvalue_2 (+ _returnvalue ScaleChange))
  (bind _returnvalue_3 (- _returnvalue ScaleChange))
  (bind _returnvalue_4 (> _maxsizepossible (.z _returnvalue_2)))
  (bind _returnvalue_5 (> _maxsizepossible (.x _returnvalue_2)))
  (bind _returnvalue_6 (> _maxsizepossible (.y _returnvalue_2)))
  (bind _returnvalue_7 (> (.x _returnvalue_3) _minsizepossible))
  (bind _returnvalue_8 (> (.y _returnvalue_3) _minsizepossible))
  (bind _returnvalue_9 (> (.z _returnvalue_3) _minsizepossible))
  (bind _returnvalue_10 (Math|Boolean|ANDBoolean _returnvalue_5 _returnvalue_6 _returnvalue_4))
  (bind _returnvalue_11 (Math|Boolean|ANDBoolean _returnvalue_7 _returnvalue_8 _returnvalue_9))
  (if Add?
    (if _returnvalue_10
      (Transformation|SetRelativeScale3D (Variables|Default|GetVisual) (Math|Vector|MakeVector (.x _returnvalue_2) (.y _returnvalue_2) (.z _returnvalue_2))))
    (return (not _returnvalue_10))
    (else
      (if _returnvalue_11
        (Transformation|SetRelativeScale3D (Variables|Default|GetVisual) (Math|Vector|MakeVector (.x _returnvalue_3) (.y _returnvalue_3) (.z _returnvalue_3))))
      (return (not _returnvalue_11)))))

(fn SetCharged
  (params (Charged? :type Boolean))
  (Variables|Default|SetIsCharged? Charged?))