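; IPlayer is a Blueprint Interface that defines how other objects talk to the player without casting to its class.
; Its setter functions push movement limits, external velocity, visual scale, charge and helium state, plus level startup transforms and death.
; Its getters expose speed, scale bounds, charged and alive status, and the player's controller, camera and game mode reference.
; All functions are empty signatures, leaving behavior to the implementing Blueprint.
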(fn UpdateZDistance
  (params (New%20Base%20Position :type Float%20%28single-precision%29) (New%20Max%20Position :type Float%20%28single-precision%29)))

(fn UpdateVisualScale
  (params (Scale%20Change :type ScaleChangeType%20Enum :default "NewEnumerator0") (ScaleChange :type Float%20%28single-precision%29))
  (return false))

(fn SetCharged
  (params (Charged? :type Boolean)))

(fn UpdateMaxSpeed
  (params (NewMaxSpeed :type Float%20%28single-precision%29)))

(fn UpdateExternalSpeed
  (params (Velocity :type Vector)))

(fn GetMaxSpeed
  (return 0.0))

(fn KillPlayer)

(fn GetIsCharged
  (return false))

(fn LockUpDownMovment
  (params (canControUpDown? :type Boolean) (NewDirection :type Integer)))

(fn GetPlayerControler
  (return 0))

(fn SetGameModeRef
  (params (GM :type My%20Game%20Mode%20Object%20Reference)))

(fn GetGameModeRef
  (return 0))

(fn UpdateHelium
  (params (HasHelium? :type Boolean)))

(fn NewLevelStartup
  (params (Position :type Vector) (Rotation :type Rotator) (Scale :type Float%20%28single-precision%29)))

(fn GetMinScale
  (return 0.0))

(fn GetMaxScale
  (return 0.0))

(fn GetPlayerCamera
  (return 0))

(fn GetIsAlive
  (return false))